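; Enemy Blueprint (orc walk animation) that wanders the navmesh and chases pawns it sees.
; Wandering chains AI MoveTo calls to random reachable points nearby, repeating on each success.
; PawnSensing sightings start a chase, with a DoOnce switching to the running animation and faster speed.
; A retriggerable delay detects lost sight, then restores walking, resets the DoOnce and resumes wandering.
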(event OnSeePawn(PawnSensing)
  (params (Pawn :type Pawn%20Object%20Reference))
  (Utilities|FlowControl|Sequence
    (:then_0
      (Utilities|FlowControl|DoOnce false
        (:Completed
          (Components|Animation|PlayAnimation (Variables|Character|GetMesh) "/Game/IA/mesh/Running__1_.Running__1_" true)
          (Variables|/Script/Engine.CharacterMovementComponent|SetMaxWalkSpeed (Variables|Character|GetCharacterMovement) 6e+02))))
    (:then_1
      (AI|AIMoveTo self "0, 0, 0" Pawn 5.0 false
        (:then
          (Utilities|FlowControl|RetriggerableDelay 2.0)
          (Components|Animation|PlayAnimation (Variables|Character|GetMesh) "/Game/IA/mesh/Orc_Walk__2_.Orc_Walk__2_" true)
          (Variables|/Script/Engine.CharacterMovementComponent|SetMaxWalkSpeed (Variables|Character|GetCharacterMovement) 3.5e+02)
          (CallFunction|Cansprintagain)
          (CallFunction|MovetoRandomLocation))))))

(event Custom|Move%20to%20random%20location
  (bind _randomlocation (Class|NavigationSystemV1|GetRandomLocationinNavigableRadius (Transformation|GetActorLocation) 1e+03 0 0))
  (AI|AIMoveTo self _randomlocation 0 5.0 false
    (:OnSuccess
      (CallFunction|MovetoRandomLocation))))

(event Custom|Cansprintagain
  (Utilities|FlowControl|DoOnce false) ; enters at Reset
)

(event EventBeginPlay
  (CallFunction|MovetoRandomLocation))

(fn ConstructionScript)